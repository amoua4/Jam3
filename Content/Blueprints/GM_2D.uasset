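; 2D game mode that runs the intro and the automatic slow-motion "Witchtime" cycle.
; BeginPlay creates the HUD, shows the logo with input disabled, then steps through timed voiced dialogue, focusing the camera on each speaker, before switching music.
; After the intro, Tick alternates cooldown and Witchtime, using timelines to ramp global time dilation while toggling HUD selection mode and notifying via WitchtimeTrigger.
; SlowHighlight briefly slows time on a focused actor outside Witchtime; Gameover is empty.
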(event `self.ReceiveBeginPlay`
  (bind _intro_dialogue (`self.Intro Dialogue`))
  (bind _dialogie_index (`self.Dialogie Index`))
  (bind (_output_character _output_text _output_time _output_timeuntilnext _output_dialogueva) (break `/Game/Blueprints/Struct_Dialogue` (`|GetArrayItem` _intro_dialogue _dialogie_index)))
  (`|ExecutionSequence`
    (:`then_0`
      (bind _returnvalue (`|CreateWidget` "/Game/Widget/UI_Player.UI_Player_C"))
      (`UserWidget.AddToViewport` _returnvalue 0)
      (set `self.HUD_ref` _returnvalue))
    (:`then_1`
      (`WidgetBlueprintLibrary.SetInputMode_GameOnly` (`GameplayStatics.GetPlayerController` 0)))
    (:`then_2`
      (`self.DisableInput` (`GameplayStatics.GetPlayerPawn` 0) (`GameplayStatics.GetPlayerController` 0))
      (bind _returnvalue_2 (`|CreateWidget` "/Game/Widget/UI_Logo.UI_Logo_C"))
      (`UserWidget.AddToViewport` _returnvalue_2 0)
      (`KismetSystemLibrary.Delay` 7.0)
      (`/Game/Widget/UI_Player.Show Intro` (`self.HUD_ref`))
      (`self.EnableInput` (`GameplayStatics.GetPlayerPawn` 0) (`GameplayStatics.GetPlayerController` 0))
      (`KismetSystemLibrary.Delay` 1.0)
      ;[1 0.07081 0.8876] Fuck you(tm) dialogue
      (if (< _dialogie_index (`KismetArrayLibrary.Array_Length` _intro_dialogue)) :!label _label
        (bind _asgs_2d (cast `/Game/Blueprints/GS_2D` (`GameplayStatics.GetGameState`)))
        (for _array_element (`/Game/Blueprints/GS_2D.AllCharacters_ref` _asgs_2d)
          (if (`|EnumEquality` (`/Game/Blueprints/BP_BaseCharacter.Character` _array_element) _output_character)
            (`/Game/Blueprints/Player/BP_Camera.Focus Actor` (`self.Camera_ref`) _array_element)
            (`/Game/Widget/UI_CharacterStats.Intro Dialogue` (cast `/Game/Widget/UI_CharacterStats` (`/Game/Blueprints/BP_BaseCharacter.UI_ref` _array_element) :!pure true) _output_text _output_time)
            (`GameplayStatics.PlaySoundAtLocation` _output_dialogueva (`self.K2_GetActorLocation` _array_element) (struct) 1.0 1.0 0.0 "/Game/Sounds/NewSoundAttenuation.NewSoundAttenuation" null null null)
            (break)))
        (`/Engine/EditorBlueprintResources/StandardMacros.IncrementInt` (`self.Dialogie Index`)
          (:`  `
            (bind _returnvalue_3 (`KismetSystemLibrary.K2_SetTimer` null "Next Dialogue" _output_timeuntilnext))
            (set `self.Dialogue Timer` _returnvalue_3)))
        (else
          (set `self.Intro` false)
          (`/Game/Widget/UI_Player.Finish Intro` (`self.HUD_ref`))
          (set `/Game/Blueprints/Player/BP_Camera.Focus` false (`self.Camera_ref`))
          (`AudioComponent.FadeOut` (`self.BGM`) 1.0 0.0 "Linear")
          (bind _returnvalue_4 (`GameplayStatics.SpawnSound2D` "/Game/Sounds/BGM/malfunction_loop_Cue.malfunction_loop_Cue" 1.0 1.0 0.0 null))
          (set `self.BGM` _returnvalue_4))))
    (:`then_3`
      (bind _returnvalue_5 (`GameplayStatics.SpawnSound2D` "/Game/Sounds/BGM/acquiescence_intro_Cue.acquiescence_intro_Cue" 1.0 1.0 0.0 null))
      (set `self.BGM` _returnvalue_5))
    (:`then_4`
      (`KismetSystemLibrary.ExecuteConsoleCommand` "disableallscreenmessages" null))))

(event `Next Dialogue`
  (bind _dialogue_timer (`self.Dialogue Timer`))
  (if (`KismetSystemLibrary.K2_IsTimerActiveHandle` _dialogue_timer)
    (`KismetSystemLibrary.K2_ClearAndInvalidateTimerHandle` _dialogue_timer)
    (goto _label)
    (else
      (goto _label))))

(event `self.ReceiveTick`
  (params (DeltaSeconds :type "Float (single-precision)"))
  (if (not (`self.Intro`))
    (`|ExecutionSequence`
      (:`then_0`
        (if (`self.WitchtimeEnable`)
          (bind _output_get (set `self.Witchtime` (`KismetMathLibrary.FMax` (- (`self.Witchtime`) (* DeltaSeconds 1.0)))))
          (if (<= _output_get 0.0)
            (`self.Exit Witchtime`))
          (else
            ;[0.1121 1 0.1281] Adding Cooldown
            (bind _output_get_2 (set `self.Cooldown` (`KismetMathLibrary.FMax` (- (`self.Cooldown`) (* DeltaSeconds 1.0)))))
            (`|ExecutionSequence`
              (:`then_0`
                (if (<= _output_get_2 0.0)
                  (`self.Enter Witchtime`))))))))))

(event `Enter Witchtime`
  (set `self.WitchtimeEnable` true)
  (set `self.Cooldown` (`self.MaxCooldown`))
  (`self.WitchtimeTrigger` true)
  (`/Game/Widget/UI_Player.Selecting Mode` (`self.HUD_ref`) true)
  (bind (_direction _newtrack_0) (`Timeline|Timeline` :!via `PlayFromStart` :!label _label_2)
    (:`Update`
      (`GameplayStatics.SetGlobalTimeDilation` (`KismetMathLibrary.Lerp` 1.0 0.05 _newtrack_0)))))

(event `Exit Witchtime`
  (set `self.WitchtimeEnable` false)
  (set `self.Witchtime` (`self.MaxWitchtime`))
  (`self.WitchtimeTrigger` false)
  (`/Game/Widget/UI_Player.Selecting Mode` (`self.HUD_ref`) false)
  (goto _label_2 :!via `ReverseFromEnd`))

(event `Slow Highlight`
  (params (Actor :type "Actor Object Reference"))
  ;[1 1 1] Slowmo Highlight
  (if (not (`self.WitchtimeEnable`))
    (`/Game/Blueprints/Player/BP_Camera.Focus Actor` (`self.Camera_ref`) Actor)
    (bind (_direction _newtrack_0) (`Timeline|Slowdown` :!via `PlayFromStart`)
      (:`Update`
        (`GameplayStatics.SetGlobalTimeDilation` (`KismetMathLibrary.Lerp` 0.2 1.0 _newtrack_0)))
      (:`Finished`
        (`KismetSystemLibrary.RetriggerableDelay` 0.6)
        (set `/Game/Blueprints/Player/BP_Camera.Focus` false (`self.Camera_ref`))))))

(event `Gameover`)

(fn `UserConstructionScript`)