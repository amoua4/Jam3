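; Mage character with four actions: Explosion, Vine Snare, Teleport and Defend.
; BeginPlay spawns a BP_MageSpell helper, which runs both attacks on a random GS_2D enemy after a cast animation and delay, with Vine Snare aimed at the floor beneath it.
; Teleport swaps places with a random character other than boss and mage, using scale timelines on the mage and particle bursts.
; Defend only sets a flag.
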(event `self.Action0`
  (bind _mage_spell (`self.Mage Spell`))
  ;[1 0 0.003604] Explosion
  (`self.Play Animation` "/Game/Sprites/Mage/Cast/mage_cast.mage_cast")
  (`KismetSystemLibrary.Delay` 0.8)
  (bind _output_get (set `self.Random Target` (`KismetArrayLibrary.Array_Random` (`/Game/Blueprints/GS_2D.Enemies_ref` (cast `/Game/Blueprints/GS_2D` (`GameplayStatics.GetGameState`) :!pure true)))))
  (set `/Game/Blueprints/AIPlayer/BP_MageSpell.Target Location` (`self.K2_GetActorLocation` _output_get) _mage_spell)
  (set `/Game/Blueprints/AIPlayer/BP_MageSpell.Target` _output_get _mage_spell)
  (`/Game/Blueprints/AIPlayer/BP_MageSpell.Explosion Attack` _mage_spell))

(event `self.ReceiveBeginPlay`
  (`parent.ReceiveBeginPlay`)
  (bind _returnvalue (`|SpawnActorFromClass` "/Game/Blueprints/AIPlayer/BP_MageSpell.BP_MageSpell_C" (`KismetMathLibrary.MakeTransform` (0.0 0.0 0.0)) "Undefined" "OverrideRootScale" null self null))
  (set `self.Mage Spell` _returnvalue))

(event `self.Action1`
  (bind _mage_spell (`self.Mage Spell`))
  ;[0 1 0.05902] Vine Snare
  (`self.Play Animation` "/Game/Sprites/Mage/Cast/mage_cast.mage_cast")
  (`KismetSystemLibrary.Delay` 0.8)
  (bind _output_get (set `self.Random Target` (`KismetArrayLibrary.Array_Random` (`/Game/Blueprints/GS_2D.Enemies_ref` (cast `/Game/Blueprints/GS_2D` (`GameplayStatics.GetGameState`) :!pure true)))))
  (set `/Game/Blueprints/AIPlayer/BP_MageSpell.Target Location` (`.ImpactPoint` (`GameplayStatics.BreakHitResult` (`.HitResult` (break `FindFloorResult` (`CharacterMovementComponent.K2_FindFloor` (`Character.CharacterMovement` _output_get) (`SceneComponent.K2_GetComponentLocation` (`Character.CapsuleComponent` _output_get))))))) _mage_spell)
  (set `/Game/Blueprints/AIPlayer/BP_MageSpell.Target` _output_get _mage_spell)
  (`/Game/Blueprints/AIPlayer/BP_MageSpell.Vine Attack` _mage_spell))

(event `self.Action2`
  ;[1 0.6382 0] Teleport
  (`self.Play Animation` "/Game/Sprites/Mage/Cast/mage_cast.mage_cast")
  (`KismetSystemLibrary.Delay` 0.8)
  (bind _asgs_2d (cast `/Game/Blueprints/GS_2D` (`GameplayStatics.GetGameState`)))
  (for _array_element (`/Game/Blueprints/GS_2D.AllCharacters_ref` _asgs_2d)
    (bind _returnvalue (`KismetStringLibrary.Conv_ObjectToString` _array_element))
    (if (and (`KismetStringLibrary.NotEqual_StrStr` (`self.Boss Name`) _returnvalue) (`KismetStringLibrary.NotEqual_StrStr` (`self.Mage Name`) _returnvalue))
      (`KismetArrayLibrary.Array_Add` (`self.TeleportTargets`) _array_element)))
  (bind _output_get (set `self.Random Target` (`KismetArrayLibrary.Array_Random` (`self.TeleportTargets`))))
  (bind (_direction _blip_out) (`Timeline|Blip Out` :!via `PlayFromStart`)
    (:`Update`
      (`self.SetActorRelativeScale3D` _blip_out))
    (:`Finished`
      (`self.Swap Places` _output_get)
      (`GameplayStatics.SpawnEmitterAtLocation` "/Game/RealtimePixelVFX/FX/legacy/P_MeshRespawn2.P_MeshRespawn2" (- (`self.K2_GetActorLocation` _output_get) (0.0 0.0 25.0)))
      (`GameplayStatics.SpawnEmitterAtLocation` "/Game/RealtimePixelVFX/FX/legacy/P_MeshRespawn2.P_MeshRespawn2" (- (`self.K2_GetActorLocation`) (0.0 0.0 25.0)))
      (bind (_direction_2 _blip_in) (`Timeline|Blip In` :!via `PlayFromStart`)
        (:`Update`
          (`self.SetActorRelativeScale3D` _blip_in))
        (:`Finished`
          (`KismetArrayLibrary.Array_Clear` (`self.TeleportTargets`)))))))

(event `self.Action3`
  ;[0 0.136 1] Defend
  (set `self.Is_Defend` true))

(event `Swap Places`
  (params (Ally :type "/Game/Blueprints/BP_BaseCharacter Object Reference"))
  ;[0.5547 0.5547 0.5547] Swap Places
  (bind _output_get (set `self.Old Position` (`self.K2_GetActorLocation`)))
  (`self.K2_SetActorLocation` (`self.K2_GetActorLocation` Ally) false true)
  (`self.K2_SetActorLocation` Ally _output_get false true)
  (`KismetSystemLibrary.PrintString` "Finsihed Swapping"))

(fn `NewFunction_0`)

(fn `UserConstructionScript`
  (`parent.UserConstructionScript`))