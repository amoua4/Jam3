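; Spell effect actor for a mage (Parent) that moves to TargetLocation and damages Target using the mage's Attack.
; ExplosionAttack activates hint and explosion particles, lowers the explosion along a timeline, then deals delayed damage.
; VineAttack slows the target, plays a snare flipbook, deals damage, then sets walk speed to a fixed value.
; Both trigger GM_2D's SlowHighlight before damage; PlayAnimation hides the sprite via retriggerable delay.
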(event `Explosion Attack`
  (bind _target (`self.Target`))
  (bind _parent (`self.Parent`))
  ;[1 0.02466 0] Explosion Spell
  (`self.K2_SetActorLocation` (`self.Target Location`) false true)
  (`|ExecutionSequence`
    (:`then_0`
      (`ActorComponent.SetActive` (`self.P_ExplodeHint`) true false)
      (bind (_direction _newtrack_0) (`Timeline|Timeline` :!via `PlayFromStart`)
        (:`Update`
          (`SceneComponent.K2_SetWorldLocation` (`self.P_Explosion`) (+ (`SceneComponent.K2_GetComponentLocation` (`self.DefaultSceneRoot`)) (`KismetMathLibrary.MakeVector` 0.0 0.0 (`KismetMathLibrary.Lerp` 100.0 20.0 _newtrack_0))) false false))))
    (:`then_1`
      (`ActorComponent.SetActive` (`self.P_Explosion`) true false)
      (`KismetSystemLibrary.Delay` 2.0)
      (`/Game/Blueprints/GM_2D.Slow Highlight` (cast `/Game/Blueprints/GM_2D` (`GameplayStatics.GetGameMode`) :!pure true) (`self.Target`))
      (`GameplayStatics.ApplyDamage` _target (`/Game/Blueprints/BP_BaseCharacter.Attack` _parent) (`Pawn.GetController` _parent) _parent "/Script/Engine.DamageType")
      (`self.SetActorScale3D` (1.0 1.0 1.0))
      (`KismetSystemLibrary.PrintString` (`KismetSystemLibrary.GetDisplayName` _target)))))

(event `Vine Attack`
  (bind _parent (`self.Parent`))
  ;[0.1335 1 0] Vine Spell
  (set `CharacterMovementComponent.MaxWalkSpeed` 10.0 (`Character.CharacterMovement` (`self.Target`)))
  (`self.K2_SetActorLocation` (+ (`self.Target Location`) (0.0 0.0 50.0)) false true)
  (`self.Play Animation` "/Game/Sprites/Mage/VineSnare/mage_vine_snare.mage_vine_snare")
  (`KismetSystemLibrary.Delay` 0.45)
  (`/Game/Blueprints/GM_2D.Slow Highlight` (cast `/Game/Blueprints/GM_2D` (`GameplayStatics.GetGameMode`) :!pure true) (`self.Target`))
  (`KismetSystemLibrary.Delay` 0.05)
  (`GameplayStatics.ApplyDamage` (`self.Target`) (`/Game/Blueprints/BP_BaseCharacter.Attack` _parent) (`Pawn.GetController` _parent) _parent "/Script/Engine.DamageType")
  (`SceneComponent.SetRelativeScale3D` (`self.Sprite`) (3.0 3.0 3.0))
  (`KismetSystemLibrary.Delay` 0.2)
  (set `CharacterMovementComponent.MaxWalkSpeed` 100.0 (`Character.CharacterMovement` (`self.Target`))))

(event `Play Animation`
  (params (NewFlipbook :type "PaperFlipbook Object Reference"))
  ;[1 0.8817 0.01873] Play Animation
  (set `self.AnimationPlaying` true)
  (`SceneComponent.SetHiddenInGame` (`self.Sprite`) false false)
  (`PaperFlipbookComponent.SetFlipbook` (`self.Sprite`) NewFlipbook)
  (`KismetSystemLibrary.RetriggerableDelay` (`PaperFlipbook.GetTotalDuration` NewFlipbook))
  (set `self.AnimationPlaying` false)
  (`SceneComponent.SetHiddenInGame` (`self.Sprite`) true false))

(fn `UserConstructionScript`)