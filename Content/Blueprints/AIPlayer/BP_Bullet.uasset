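; BP_Bullet is a homing projectile that damages the boss.
; On BeginPlay it takes the first entry of the GS_2D game state's EnemiesRef and sets that boss's capsule as its ProjectileMovement homing target.
; Its sphere overlap ignores other bullets, and on hitting a boss calls EventNormalDamage with fixed damage and destroys the bullet.
; An ApplyDamage node is left unconnected and never runs.
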(event `self.ReceiveBeginPlay`
  (bind _asbp_boss (cast `/Game/Blueprints/Boss/BP_Boss` (`|GetArrayItem` (`/Game/Blueprints/GS_2D.Enemies_ref` (cast `/Game/Blueprints/GS_2D` (`GameplayStatics.GetGameState`) :!pure true)))))
  (set `ProjectileMovementComponent.HomingTargetComponent` (`Character.CapsuleComponent` _asbp_boss) (`self.ProjectileMovement`)))

(event `self.Sphere1.OnComponentBeginOverlap`
  (params (OverlappedComponent :type "PrimitiveComponent Object Reference") (OtherActor :type "Actor Object Reference") (OtherComp :type "PrimitiveComponent Object Reference") (OtherBodyIndex :type Integer) (bFromSweep :type Boolean) (SweepResult :type "HitResult Structure (by ref)"))
  (cast `/Game/Blueprints/AIPlayer/BP_Bullet` OtherActor
    (:`CastFailed`
      (bind _asbp_boss (cast `/Game/Blueprints/Boss/BP_Boss` OtherActor))
      (`/Game/Blueprints/BP_BaseCharacter.Event NormalDamage` _asbp_boss 100.0 null)
      (`self.K2_DestroyActor`))))

(fn `UserConstructionScript`)