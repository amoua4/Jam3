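; AI melee Warrior party member that fights the boss with a randomly delayed auto attack and four actions.
; Flurry, fade slash and giga slash time launches, animations, effects and pathing changes with delays; fade slash and the fourth action set defending.
; Attacks share a Slash sphere trace toward the first enemy, using Cast to choose normal damage or slow-highlighted heavy damage.
; BeginPlay calls Killed right after the parent's setup.
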(event `self.ReceiveBeginPlay`
  (`parent.ReceiveBeginPlay`)
  (`self.Killed`))

(event `self.AutoAttack`
  (bind _returnvalue (`self.K2_GetActorLocation`))
  (bind _returnvalue_2 (`self.K2_GetActorLocation`))
  (bind _p_normalslah (`self.P_NormalSlah`))
  (if (not (`self.Is_Dead`))
    (`KismetSystemLibrary.Delay` (`KismetMathLibrary.RandomFloatInRange` 0.0 0.4))
    (if (> (`self.Cast`) 1.5)
      (bind (_outhit _returnvalue_3) (`KismetSystemLibrary.SphereTraceSingle` :`Start` _returnvalue :`End` _returnvalue :`Radius` 120.0 :`TraceChannel` "TraceTypeQuery4" :`TraceColor` (struct :`R` 1.0 :`G` 0.106359 :`A` 1.0) :`TraceHitColor` (struct :`G` 0.495251 :`B` 1.0 :`A` 1.0) :`DrawTime` 0.5))
      (if _returnvalue_3
        (`self.Launch Character to Boss` 100.0)
        (`self.Play Animation` "/Game/Sprites/Warrior/Auto/warrior_auto.warrior_auto")
        (`KismetSystemLibrary.Delay` 0.2)
        (`NiagaraFunctionLibrary.SpawnSystemAtLocation` "/Game/RealtimePixelVFX/FX/P_NormalSlah.P_NormalSlah" (`SceneComponent.K2_GetComponentLocation` _p_normalslah) (`SceneComponent.K2_GetComponentRotation` _p_normalslah))
        ;[1 1 1] Slash
        (bind (_outhit_2 _returnvalue_4) (`KismetSystemLibrary.SphereTraceSingle` :`Start` _returnvalue_2 :`End` (+ _returnvalue_2 (* (`KismetMathLibrary.GetForwardVector` (`KismetMathLibrary.FindLookAtRotation` _returnvalue_2 (`self.K2_GetActorLocation` (`|GetArrayItem` (`/Game/Blueprints/GS_2D.Enemies_ref` (cast `/Game/Blueprints/GS_2D` (`GameplayStatics.GetGameState`) :!pure true)))))) 100.0)) :`Radius` 100.0 :`TraceChannel` "TraceTypeQuery4" :`TraceColor` (struct :`R` 1.0 :`G` 0.106359 :`A` 1.0) :`TraceHitColor` (struct :`G` 0.495251 :`B` 1.0 :`A` 1.0) :`DrawTime` 0.5 :!label _label))
        (if _returnvalue_4
          (if (<= (`self.Cast`) 0.0)
            (`/Game/Blueprints/GM_2D.Slow Highlight` (cast `/Game/Blueprints/GM_2D` (`GameplayStatics.GetGameMode`) :!pure true) self)
            (bind (_bblockinghit _binitialoverlap _time _distance _location _impactpoint _normal _impactnormal _physmat _hitactor) (`GameplayStatics.BreakHitResult` _outhit_2))
            (bind _asbp_boss (cast `/Game/Blueprints/Boss/BP_Boss` _hitactor))
            (`GameplayStatics.ApplyDamage` _asbp_boss 350.0 (`self.GetController`) self "/Script/Engine.DamageType")
            (else
              (bind _asbp_boss_2 (cast `/Game/Blueprints/Boss/BP_Boss` _hitactor))
              (`self.Event NormalDamage` _asbp_boss_2 100.0 self))))))))

(event `Slash`
  ;[1 1 1] Slash
  (goto _label))

(event `self.Action0`
  (bind _p_normalslah (`self.P_NormalSlah`))
  (bind _p_normalslah_2 (`self.P_NormalSlah`))
  (set `self.CurrentPathing` "NewEnumerator0")
  (`self.Launch Character to Boss` 600.0)
  (`self.Play Animation` "/Game/Sprites/Warrior/Flurry/warrior_flurry.warrior_flurry")
  (`KismetSystemLibrary.Delay` 0.6)
  (`self.Launch Character to Boss` 300.0)
  (`ActorComponent.SetActive` (`self.P_SpecialSlash`) true false)
  (`self.Slash`)
  (`KismetSystemLibrary.Delay` 0.3)
  (`self.Launch Character to Boss` 300.0)
  (`NiagaraFunctionLibrary.SpawnSystemAtLocation` "/Game/RealtimePixelVFX/FX/P_NormalSlah.P_NormalSlah" (`SceneComponent.K2_GetComponentLocation` _p_normalslah_2) (`SceneComponent.K2_GetComponentRotation` _p_normalslah_2))
  (`self.Slash`)
  (`KismetSystemLibrary.Delay` 0.5)
  (`self.Launch Character to Boss` 300.0)
  (`self.Slash`)
  (`NiagaraFunctionLibrary.SpawnSystemAtLocation` "/Game/RealtimePixelVFX/FX/P_NormalSlah.P_NormalSlah" (`SceneComponent.K2_GetComponentLocation` _p_normalslah) (`SceneComponent.K2_GetComponentRotation` _p_normalslah))
  (`KismetSystemLibrary.Delay` 0.3)
  (set `self.CurrentPathing` "NewEnumerator1"))

(event `self.Action1`
  (bind _p_normalslah (`self.P_NormalSlah`))
  ;[1 1 1] Fade Slash
  (set `self.CurrentPathing` "NewEnumerator0")
  (`self.Play Animation` "/Game/Sprites/Warrior/FadingSlash/warrior_fading_slash.warrior_fading_slash")
  (`KismetSystemLibrary.Delay` 0.1)
  (`self.Slash`)
  (`NiagaraFunctionLibrary.SpawnSystemAtLocation` "/Game/RealtimePixelVFX/FX/P_NormalSlah.P_NormalSlah" (`SceneComponent.K2_GetComponentLocation` _p_normalslah) (`SceneComponent.K2_GetComponentRotation` _p_normalslah))
  (`KismetSystemLibrary.Delay` 0.1)
  (`self.Launch Character to Boss` -500.0)
  (`KismetSystemLibrary.Delay` 0.3)
  (set `self.CurrentPathing` "NewEnumerator2")
  (set `self.Is_Defend` true))

(event `self.Action2`
  ;[1 0.8821 0] Giga Slash
  (set `self.CurrentPathing` "NewEnumerator0")
  (`self.Launch Character to Boss` 600.0)
  (`self.Play Animation` "/Game/Sprites/Warrior/GigaSlash/warrior_giga_slash.warrior_giga_slash")
  (`KismetSystemLibrary.Delay` 0.8)
  (`self.Slash`)
  (`ActorComponent.SetActive` (`self.P_GigaSlash`) true false)
  (`KismetSystemLibrary.Delay` 0.2)
  (set `self.CurrentPathing` "NewEnumerator2"))

(event `self.Action3`
  ;[0.1859 1 0] Action 3
  (set `self.Is_Defend` true))

(fn `UserConstructionScript`
  (`parent.UserConstructionScript`))