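; AI-controlled party member for a boss fight, which registers itself in GS_2D and chooses its own actions.
; ThinkAction makes a weighted random pick from DT_Actions chances, based on whether the boss is party-wiping or this ally holds aggro.
; Command overrides the queued action while Patience is below its maximum, raising Patience each time.
; The looping Fire timer is empty; attack, movement and slow-motion logic are disconnected.
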(event `self.ReceiveBeginPlay`
  (`parent.ReceiveBeginPlay`)
  (`|ExecutionSequence`
    (:`then_0`
      (`KismetSystemLibrary.K2_SetTimer` null "Fire" 0.2 true))
    (:`then_1`
      ;[1 1 1] Add Ref to GS
      (bind _asgs_2d (cast `/Game/Blueprints/GS_2D` (`GameplayStatics.GetGameState`)))
      (`KismetArrayLibrary.Array_Add` (`/Game/Blueprints/GS_2D.AIPlayers_ref` _asgs_2d) self))
    (:`then_2`
      (`self.Think Action`))))

(event `self.ReceiveTick`
  (params (DeltaSeconds :type "Float (single-precision)"))
  (`parent.ReceiveTick` DeltaSeconds))

(event `self.Think Action`
  (bind _asgs_2d (cast `/Game/Blueprints/GS_2D` (`GameplayStatics.GetGameState`) :!pure true))
  ;[1 1 1] Think Action
  (`parent.Think Action`)
  (set `self.CurrentAction` "NewEnumerator4")
  (if (`|EnumEquality` (`self.QueueAction`) "NewEnumerator4")
    (`KismetArrayLibrary.Array_Clear` (`self.ActionWeights`))
    (set `self.hasAggro` true)
    ;;[1 1 1] Check if this have aggro
    (bind _max_aggro_player (`/Game/Blueprints/GS_2D.Find Max Aggro` _asgs_2d))
    (set `self.hasAggro` (== _max_aggro_player self))
    ;;[1 1 1] Is the boss doing a Party Wipe?
    (set `self.bossDoingPartyWipe` (`|EnumEquality` (`/Game/Blueprints/BP_BaseCharacter.CurrentAction` (`|GetArrayItem` (`/Game/Blueprints/GS_2D.Enemies_ref` _asgs_2d))) "NewEnumerator2"))
    ;;[1 1 1] Figure out weights for each action option
    (for _index (range 4)
      (bind _returnvalue (`|GetDataTableRow` "/Game/Blueprints/DT_Actions.DT_Actions" (`KismetStringLibrary.Conv_StringToName` (`KismetStringLibrary.Concat_StrStr` (`|GetEnumeratorNameAsString` (`self.Character`)) ":" (`KismetStringLibrary.Conv_IntToString` _index))))
        (:`then`
          (if (`self.bossDoingPartyWipe`)
            (set `self.actionUseChance` (`.AllyUseChance_PartyWipe_23_3FE01D102741D808FC424D874A307A75` (break `/Game/Blueprints/Struct_Actions` _returnvalue)))
            (elif (`self.hasAggro`)
              (set `self.actionUseChance` (`.AllyUseChance_HasAggro_19_8937B8D0C14B1A1E11F82189CC9CB01E` (break `/Game/Blueprints/Struct_Actions` _returnvalue)))
              (else
                (set `self.actionUseChance` (`.AllyUseChance_NoAggro_21_4EE7C7778A4BE8839E554CAACFFC1A5B` (break `/Game/Blueprints/Struct_Actions` _returnvalue))))))
          (for _ (range (+ (`KismetMathLibrary.FTrunc` (* (`self.actionUseChance`) 100.0)) 1))
            (`KismetArrayLibrary.Array_Add` (`self.ActionWeights`) _index)))))
    ;;[1 1 1] Pick an action
    (bind _output_get (set `self.QueueAction` (cast `/Game/Blueprints/Enum_Action` (`KismetMathLibrary.Conv_IntToByte` (`KismetArrayLibrary.Array_Random` (`self.ActionWeights`))))))
    (`KismetSystemLibrary.PrintString` (`|GetEnumeratorNameAsString` _output_get))
    (message `/Game/Widget/BPInter_Widget.Fire Dialogue` (`self.UI_ref`) false)))

(event `/Game/Blueprints/Inter_AIPlayer.Command`
  (params (`New Action` :type "/Game/Blueprints/Enum_Action Enum" :default "NewEnumerator0"))
  ;[0.2619 1 0.2312] Command
  (if (`|EnumInequality` `New Action` (`self.QueueAction`))
    (message `/Game/Widget/BPInter_Widget.Fire Dialogue` (`self.UI_ref`) true)
    (if (< (`self.Patience`) (`self.MaxPatience`))
      (set `self.QueueAction` `New Action`)
      (`self.Add Patience` 30.0))))

(event `Fire`
  ;[1 0.873 0.2384] Stupid Fire
)

(fn `UserConstructionScript`)