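; Base 2D character for a cooldown-driven turn combat game, shared by Support, Mage, Tank and Boss types.
; BeginPlay fills stats, tints the sprite by type, links its widget and registers non-boss characters with the HUD.
; Tick fills a cooldown that ends the turn when full, then promotes the queued action and re-thinks shortly into the next cycle.
; ThinkAction, TurnEnd and FireAction are empty hooks; getters expose state.
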(event `self.ReceiveBeginPlay`
  (`|ExecutionSequence`
    (:`then_0`
      ;[0.9769 0.2077 1] Set reference for UI
      (bind _asui_character (cast `/Game/Widget/UI_Character` (`WidgetComponent.GetWidget` (`self.Widget`))))
      (set `/Game/Widget/UI_Character.Actor` self _asui_character)
      (`self.Think Action`))
    (:`then_1`
      ;[1 0.05185 0.07175] Reset Cooldown and Health
      (set `self.Cooldown` (`self.MaxCooldown`))
      (set `self.Health` (`self.MaxHealth`)))
    (:`then_2`
      ;[1 1 1] Hint Color
      (`PaperFlipbookComponent.SetSpriteColor` (`self.Sprite`) (select `/Game/Blueprints/Enum_Characters` (`self.Character`) :`NewEnumerator0` (struct :`G` 1.0 :`B` 0.119255 :`A` 1.0) :`NewEnumerator1` (struct :`G` 0.389882 :`B` 1.0 :`A` 1.0) :`NewEnumerator2` (struct :`R` 1.0 :`B` 0.980125 :`A` 1.0) :`NewEnumerator3` (struct :`R` 0.630208 :`G` 0.022614 :`A` 1.0) :!type "LinearColor Structure")))
    (:`then_3`
      ;[1 1 1] Assign HUD UI
      (if (`|EnumInequality` (`self.Character`) "NewEnumerator3")
        (bind _asgm_2d (cast `/Game/Blueprints/GM_2D` (`GameplayStatics.GetGameMode`)))
        (`/Game/Widget/UI_Player.Assign UI` (`/Game/Blueprints/GM_2D.HUD_ref` _asgm_2d) self)))))

(event `self.ReceiveTick`
  (params (DeltaSeconds :type "Float (single-precision)"))
  (bind _returnvalue (+ (`self.Cooldown`) (* DeltaSeconds 1.0)))
  (`|ExecutionSequence`
    (:`then_0`
      ;[0.1121 1 0.1281] Adding Cooldown
      (bind _output_get (set `self.Cooldown` (`KismetMathLibrary.FMin` _returnvalue (`self.MaxCooldown`))))
      (`|ExecutionSequence`
        (:`then_0`
          (if (> _returnvalue (`self.MaxCooldown`))
            (`/Engine/EditorBlueprintResources/StandardMacros.DoOnce` false :!label _label
              (:`Completed`
                (`self.Reset Cooldown`)
                (`self.Turn End`)
                (set `self.turn_ended` true)
                (`|ExecutionSequence`
                  (:`then_0`
                    (goto _label :!via `Reset`))
                  (:`then_1`
                    (goto _label_2 :!via `Reset`)))))))
        (:`then_1`
          ;[1 0.5566 0] Thinking action check
          (if (>= _output_get (/ (`self.MaxCooldown`) 10.0))
            (`/Engine/EditorBlueprintResources/StandardMacros.DoOnce` false :!label _label_2
              (:`Completed`
                (set `self.turn_ended` false)
                (`self.Change Action`)
                (`self.Think Action`)))))))))

(event `Reset Cooldown`
  ;[0.394 1 0.343] Reset Cooldown
  (set `self.Cooldown` 0.0))

(event `Think Action`)

(event `Change Action`
  (set `self.CurrentAction` (`self.QueueAction`))
  (set `self.QueueAction` "NewEnumerator4"))

(event `Turn End`)

(event `Fire Action`)

(fn `Get Action`
  (returns (Action :type "/Game/Blueprints/Enum_Action Enum"))
  (return (`self.CurrentAction`)))

(fn `Get Cooldown`
  (returns (Cooldown :type "Float (double-precision)"))
  (return (`self.Cooldown`)))

(fn `Get Health`
  (returns (Health :type "Float (double-precision)"))
  (return (`self.Health`)))

(fn `Get Max Cooldown`
  (returns (`Max Cooldown` :type "Float (double-precision)"))
  (return (`self.MaxCooldown`)))

(fn `Get Max Health`
  (returns (`Max Health` :type "Float (double-precision)"))
  (return (`self.MaxHealth`)))

(fn `Get Queued Action`
  (returns (`Queued Action` :type "/Game/Blueprints/Enum_Action Enum"))
  (return (`self.QueueAction`)))

(fn `UserConstructionScript`)