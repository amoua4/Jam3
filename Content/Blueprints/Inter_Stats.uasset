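; Inter_Stats is a stats interface, judging by its name and stub functions, for querying a character's combat state.
; It declares getters for health, max health, attack and a boosted flag, plus enum getters for character, current action and queued action.
; Each function returns only a default value, so the real values must come from whatever implements it.
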(fn `Get Action`
  (returns (Action :type "/Game/Blueprints/Enum_Action Enum"))
  (return "NewEnumerator0"))

(fn `Get Attack`
  (returns (Attack :type "Float (double-precision)"))
  (return 0.0))

(fn `Get Boosted`
  (returns (Boosted :type Boolean))
  (return false))

(fn `Get Character`
  (returns (Character :type "/Game/Blueprints/Enum_Characters Enum"))
  (return "NewEnumerator0"))

(fn `Get Health`
  (returns (Health :type "Float (double-precision)"))
  (return 0.0))

(fn `Get Max Health`
  (returns (`Max Health` :type "Float (double-precision)"))
  (return 0.0))

(fn `Get Queued Action`
  (returns (`Queued Action` :type "/Game/Blueprints/Enum_Action Enum"))
  (return "NewEnumerator0"))