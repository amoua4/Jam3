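; Gameplay camera actor that blends in as player zero's view target shortly after play begins and registers itself with the GM_2D game mode.
; Each tick it sits at a fixed height, offset from the midpoint between the player pawn and the average position of the game state's AI players.
; Spring arm length eases with their 2D separation.
; FocusActor permanently switches it to follow one actor at a closer zoom.
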(event `self.ReceiveBeginPlay`
  ;[1 0 0.1875] Set view target
  (`KismetSystemLibrary.Delay` 3.0)
  (`PlayerController.SetViewTargetWithBlend` (`GameplayStatics.GetPlayerController` 0) self 6.0 "VTBlend_Cubic" 0.0 false)
  (bind _asgm_2d (cast `/Game/Blueprints/GM_2D` (`GameplayStatics.GetGameMode`)))
  (set `/Game/Blueprints/GM_2D.Camera_ref` self _asgm_2d))

(event `self.ReceiveTick`
  (params (DeltaSeconds :type "Float (single-precision)"))
  (bind _springarm (`self.SpringArm`))
  (bind _returnvalue (`self.K2_GetActorLocation` (`GameplayStatics.GetPlayerPawn` 0)))
  (bind _asgs_2d (cast `/Game/Blueprints/GS_2D` (`GameplayStatics.GetGameState`)))
  (bind _returnvalue_2 (`GameplayStatics.GetActorArrayAverageLocation` (`/Game/Blueprints/GS_2D.AIPlayers_ref` _asgs_2d)))
  (if (`self.Focus`)
    (bind _output_get (set `self.View_Location` (- (`self.K2_GetActorLocation` (`self.FocusCharacter`)) (0.0 80.0 0.0))))
    (`self.K2_SetActorLocation` (`KismetMathLibrary.MakeVector` (.x _output_get) (.y _output_get) 130.0)) ; Change this to reletive
    (else
      (bind _output_get_2 (set `self.View_Location` (- (`KismetMathLibrary.VLerp` _returnvalue_2 _returnvalue 0.5) (0.0 80.0 0.0))))
      (`self.K2_SetActorLocation` (`KismetMathLibrary.MakeVector` (.x _output_get_2) (.y _output_get_2) 130.0)) ; Change this to reletive
    ))
  (set `SpringArmComponent.TargetArmLength` (`KismetMathLibrary.FInterpTo` (`SpringArmComponent.TargetArmLength` _springarm) (`KismetMathLibrary.SelectFloat` 400.0 (`KismetMathLibrary.MapRangeClamped` (`KismetMathLibrary.Vector_Distance2D` _returnvalue_2 _returnvalue) 100.0 1000.0 500.0 800.0) (`self.Focus`)) (`GameplayStatics.GetWorldDeltaSeconds`) 20.0) _springarm))

(event `Focus Actor`
  (params (Actor :type "Actor Object Reference"))
  ;[1 1 1] Focus
  (set `self.FocusCharacter` Actor)
  (set `self.Focus` true))

(fn `UserConstructionScript`)