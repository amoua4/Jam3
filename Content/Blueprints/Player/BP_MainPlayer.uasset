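; Player-controlled healer character that moves freely outside Witchtime and, during it, navigates the HUD menu and queues abilities for itself or the selected actor.
; Ability inputs also advance intro dialogue, and StartTurn exits Witchtime.
; CastingAbility runs heal, shield, boost or haste (random if none set) on AI players overlapping the Shield component, and ThinkAction resets effects except haste.
; Older targeting and firing logic remains disconnected.
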(event `self.ReceiveBeginPlay`
  (`parent.ReceiveBeginPlay`)
  (`|ExecutionSequence`
    (:`then_0`
      ;[1 1 1] Select a target first
      (bind _asgs_2d (cast `/Game/Blueprints/GS_2D` (`GameplayStatics.GetGameState`)))
      (bind _output_get (set `self.Target` (`|GetArrayItem` (`/Game/Blueprints/GS_2D.AIPlayers_ref` _asgs_2d))))
      (set `self.SearchTarget` _output_get))))

(event `self.ReceiveTick`
  (params (DeltaSeconds :type "Float (single-precision)"))
  (`parent.ReceiveTick` DeltaSeconds))

(event `self.Witchtime Trigger`
  (params (`Witchtime Enabled` :type Boolean))
  ;[1 0 0.7697] Witchtime Trigger COmmand
  (`parent.Witchtime Trigger` `Witchtime Enabled`)
  (`self.Set Command Mode` (not `Witchtime Enabled`)))

(event `Key|Escape`
  (params (Key :type "Key Structure"))
  ;[1 1 1] Quite
  (:`Pressed`
    (`KismetSystemLibrary.QuitGame` null "Quit")))

(event `InputAxis|Move Right / Left`
  (params (AxisValue :type "Float (single-precision)"))
  ;[1 1 1] Input
  (if (`self.command_mode`)
    (`self.AddMovementInput` (1.0 0.0 0.0) AxisValue)))

(event `InputAction|MenuUp`
  (params (Key :type "Key Structure"))
  ;[1 1 1] Move Menu
  (:`Pressed`
    (if (and (not (`/Game/Blueprints/GM_2D.Intro` (cast `/Game/Blueprints/GM_2D` (`GameplayStatics.GetGameMode`) :!pure true))) (not (`self.command_mode`)))
      (bind _asgm_2d (cast `/Game/Blueprints/GM_2D` (`GameplayStatics.GetGameMode`)))
      (`/Game/Widget/UI_Player.Move Section` (`/Game/Blueprints/GM_2D.HUD_ref` _asgm_2d) true))))

(event `InputAxis|Move Forward / Backward`
  (params (AxisValue :type "Float (single-precision)"))
  ;[1 1 1] Input
  (if (`self.command_mode`)
    (`self.AddMovementInput` (0.0 1.0 0.0) (* AxisValue -1.0))))

(event `InputAction|MenuDown`
  (params (Key :type "Key Structure"))
  ;[1 1 1] Move Menu
  (:`Pressed`
    (if (and (not (`/Game/Blueprints/GM_2D.Intro` (cast `/Game/Blueprints/GM_2D` (`GameplayStatics.GetGameMode`) :!pure true))) (not (`self.command_mode`)))
      (bind _asgm_2d (cast `/Game/Blueprints/GM_2D` (`GameplayStatics.GetGameMode`)))
      (`/Game/Widget/UI_Player.Move Section` (`/Game/Blueprints/GM_2D.HUD_ref` _asgm_2d) false))))

(event `Set Command Mode`
  (params (True :type Boolean))
  ;[1 1 1] Change command mode
  (bind _output_get (set `self.command_mode` True))
  (`KismetSystemLibrary.PrintString` (`KismetTextLibrary.Conv_TextToString` (`|FormatText` "COMMAND: {mode}" _output_get)) true true (struct :`R` 1.0 :`B` 0.1104 :`A` 1.0))
  (bind _asgm_2d (cast `/Game/Blueprints/GM_2D` (`GameplayStatics.GetGameMode`)))
  (`/Game/Widget/UI_Player.Command Mode` (`/Game/Blueprints/GM_2D.HUD_ref` _asgm_2d) (`self.command_mode`)))

(event `InputAction|ActionUp`
  (params (Key :type "Key Structure"))
  ;[1 1 1] Select
  (:`Pressed`
    (bind _asgm_2d (cast `/Game/Blueprints/GM_2D` (`GameplayStatics.GetGameMode`)))
    (if (`/Game/Blueprints/GM_2D.Intro` _asgm_2d)
      (`/Game/Blueprints/GM_2D.Next Dialogue` _asgm_2d)
      (elif (not (`self.command_mode`))
        (bind _hud_ref (`/Game/Blueprints/GM_2D.HUD_ref` _asgm_2d))
        (if (!= (`/Game/Widget/UI_Player.SelectActor` _hud_ref) self)
          (message `/Game/Blueprints/Inter_AIPlayer.Command` (`/Game/Widget/UI_Player.SelectActor` _hud_ref) "NewEnumerator0")
          (elif (not (`|EnumEquality` (`self.QueueAction`) "NewEnumerator0"))
            (set `self.QueueAction` "NewEnumerator0")
            (message `/Game/Widget/BPInter_Widget.Fire Dialogue` (`self.UI_ref`) true :!label _label)
            (`GameplayStatics.PlaySound2D` "/Game/Sounds/SFX/button_Cue.button_Cue" 1.0 1.0 0.0 null null)))))))

(event `InputAction|StartTurn`
  (params (Key :type "Key Structure"))
  ;[1 0.9847 0.2568] Start Turn
  (:`Pressed`
    (bind _asgm_2d (cast `/Game/Blueprints/GM_2D` (`GameplayStatics.GetGameMode`)))
    (if (`/Game/Blueprints/GM_2D.Intro` _asgm_2d)
      (`/Game/Blueprints/GM_2D.Next Dialogue` _asgm_2d)
      (elif (and (`self.Witchtime_ref`) (`|EnumInequality` (`self.QueueAction`) "NewEnumerator4"))
        (bind _asgm_2d_2 (cast `/Game/Blueprints/GM_2D` (`GameplayStatics.GetGameMode`)))
        (`/Game/Blueprints/GM_2D.Exit Witchtime` _asgm_2d_2)))))

(event `InputAction|ActionLeft`
  (params (Key :type "Key Structure"))
  ;[1 1 1] Select
  (:`Pressed`
    (bind _asgm_2d (cast `/Game/Blueprints/GM_2D` (`GameplayStatics.GetGameMode`)))
    (if (`/Game/Blueprints/GM_2D.Intro` _asgm_2d)
      (`/Game/Blueprints/GM_2D.Next Dialogue` _asgm_2d)
      (elif (not (`self.command_mode`))
        (bind _hud_ref (`/Game/Blueprints/GM_2D.HUD_ref` _asgm_2d))
        (if (!= (`/Game/Widget/UI_Player.SelectActor` _hud_ref) self)
          (message `/Game/Blueprints/Inter_AIPlayer.Command` (`/Game/Widget/UI_Player.SelectActor` _hud_ref) "NewEnumerator1")
          (elif (not (`|EnumEquality` (`self.QueueAction`) "NewEnumerator1"))
            (set `self.QueueAction` "NewEnumerator1")
            (goto _label)))))))

(event `Healing`
  (bind _result (`BlueprintSetLibrary.Set_ToArray` (`self.AllTargets`)))
  (if (`KismetArrayLibrary.Array_IsNotEmpty` _result)
    (for _array_element _result
      (`self.Heal` _array_element 100.0))
    (`self.Play Animation` "/Game/Sprites/Healer/Idle/healer_idle.healer_idle")
    (else
      (`self.Heal` 100.0))))

(event `InputAction|ActionRight`
  (params (Key :type "Key Structure"))
  ;[1 1 1] Select
  (:`Pressed`
    (bind _asgm_2d (cast `/Game/Blueprints/GM_2D` (`GameplayStatics.GetGameMode`)))
    (if (`/Game/Blueprints/GM_2D.Intro` _asgm_2d)
      (`/Game/Blueprints/GM_2D.Next Dialogue` _asgm_2d)
      (elif (not (`self.command_mode`))
        (bind _hud_ref (`/Game/Blueprints/GM_2D.HUD_ref` _asgm_2d))
        (if (!= (`/Game/Widget/UI_Player.SelectActor` _hud_ref) self)
          (message `/Game/Blueprints/Inter_AIPlayer.Command` (`/Game/Widget/UI_Player.SelectActor` _hud_ref) "NewEnumerator2")
          (elif (not (`|EnumEquality` (`self.QueueAction`) "NewEnumerator2"))
            (set `self.QueueAction` "NewEnumerator2")
            (goto _label)))))))

(event `InputAction|ActionDown`
  (params (Key :type "Key Structure"))
  ;[1 1 1] Select
  (:`Pressed`
    (bind _asgm_2d (cast `/Game/Blueprints/GM_2D` (`GameplayStatics.GetGameMode`)))
    (if (`/Game/Blueprints/GM_2D.Intro` _asgm_2d)
      (`/Game/Blueprints/GM_2D.Next Dialogue` _asgm_2d)
      (elif (not (`self.command_mode`))
        (bind _hud_ref (`/Game/Blueprints/GM_2D.HUD_ref` _asgm_2d))
        (if (!= (`/Game/Widget/UI_Player.SelectActor` _hud_ref) self)
          (message `/Game/Blueprints/Inter_AIPlayer.Command` (`/Game/Widget/UI_Player.SelectActor` _hud_ref) "NewEnumerator3")
          (elif (not (`|EnumEquality` (`self.QueueAction`) "NewEnumerator3"))
            (set `self.QueueAction` "NewEnumerator3")
            (goto _label)))))))

(event `self.Casting Ability`
  (bind _shield (`self.Shield`))
  ;[1 1 1] Random Ability if not selected
  (if (`|EnumEquality` (`self.CurrentAction`) "NewEnumerator4")
    (set `self.CurrentAction` (`KismetArrayLibrary.Array_Random` (`|MakeArray` "NewEnumerator0" "NewEnumerator1" "NewEnumerator2" "NewEnumerator3" :!type "/Game/Blueprints/Enum_Action Enum"))))
  (`|ExecutionSequence`
    (:`then_0`
      ;[1 1 1] VA Call out
      (`GameplayStatics.SpawnSoundAttached` (select `/Game/Blueprints/Enum_Action` (`self.CurrentAction`) :`NewEnumerator0` "/Game/Sounds/VA/healer_healing.healer_healing" :`NewEnumerator1` "/Game/Sounds/VA/healer_barrier.healer_barrier" :`NewEnumerator2` "/Game/Sounds/VA/healer_boosted.healer_boosted" :`NewEnumerator3` "/Game/Sounds/VA/healer_speed.healer_speed" :!type "SoundBase Object Reference") (`self.CapsuleComponent`) "None" (0.0 0.0 0.0) (struct) "SnapToTarget" true 1.0 1.0 0.0 "/Game/Sounds/NewSoundAttenuation.NewSoundAttenuation" null))
    (:`then_1`
      (switch `/Game/Blueprints/Enum_Action` (`self.CurrentAction`)
        (:`NewEnumerator0`
          (`ActorComponent.SetActive` (`self.P_HealHint`) true false)
          (bind _returnvalue (`KismetSystemLibrary.K2_SetTimerDelegate` (delegate `Healing`) 1.0 true))
          (set `self.Healing_Timer` _returnvalue))
        (:`NewEnumerator1`
          (`SceneComponent.SetHiddenInGame` _shield false false)
          (`PrimitiveComponent.SetCollisionResponseToChannel` _shield "ECC_WorldDynamic" "ECR_Block"))
        (:`NewEnumerator2`
          (`ActorComponent.SetActive` (`self.P_BoostHint`) true false))
        (:`NewEnumerator3`
          (`ActorComponent.SetActive` (`self.P_SPeedHint`) true false))))
    (:`then_2`
      (bind _result (`BlueprintSetLibrary.Set_ToArray` (`self.AllTargets`)))
      (for _array_element _result
        (switch `/Game/Blueprints/Enum_Action` (`self.CurrentAction`)
          (:`NewEnumerator1`
            (set `/Game/Blueprints/BP_BaseCharacter.Is_Shield` true _array_element))
          (:`NewEnumerator2`
            (set `/Game/Blueprints/BP_BaseCharacter.Is_Boost` true _array_element))
          (:`NewEnumerator3`
            (set `/Game/Blueprints/BP_BaseCharacter.Is_Haste` true _array_element)))))))

(event `self.Think Action`
  (bind _shield (`self.Shield`))
  (set `self.CurrentAction` "NewEnumerator4")
  (`ActorComponent.SetActive` (`self.P_HealHint`) false false)
  (`ActorComponent.SetActive` (`self.P_SPeedHint`) false false)
  (`ActorComponent.SetActive` (`self.P_BoostHint`) false false)
  (`SceneComponent.SetHiddenInGame` _shield true false)
  (`PrimitiveComponent.SetCollisionResponseToChannel` _shield "ECC_WorldDynamic" "ECR_Ignore")
  (`KismetSystemLibrary.K2_ClearAndInvalidateTimerHandle` (`self.Healing_Timer`))
  (bind _result (`BlueprintSetLibrary.Set_ToArray` (`self.AllTargets`)))
  (for _array_element _result
    (set `/Game/Blueprints/BP_BaseCharacter.Is_Shield` false _array_element)
    (set `/Game/Blueprints/BP_BaseCharacter.Is_Boost` false _array_element)))

(event `InputAction|Lockon`
  (params (Key :type "Key Structure"))
  ;[0 0.5455 1] Select Lock on target
)

(event `InputAction|Fire`
  (params (Key :type "Key Structure"))
  ;[1 0.873 0.2384] Stupid Fire
)

(event `self.Shield.OnComponentBeginOverlap`
  (params (OverlappedComponent :type "PrimitiveComponent Object Reference") (OtherActor :type "Actor Object Reference") (OtherComp :type "PrimitiveComponent Object Reference") (OtherBodyIndex :type Integer) (bFromSweep :type Boolean) (SweepResult :type "HitResult Structure (by ref)"))
  ;[1 1 1] AOE Detection
  (bind _asbp_aiplayer (cast `/Game/Blueprints/AIPlayer/BP_AIPlayer` OtherActor))
  (`BlueprintSetLibrary.Set_Add` (`self.AllTargets`) _asbp_aiplayer)
  (switch `/Game/Blueprints/Enum_Action` (`self.CurrentAction`)
    (:`NewEnumerator1`
      (set `/Game/Blueprints/BP_BaseCharacter.Is_Shield` true _asbp_aiplayer))
    (:`NewEnumerator2`
      (set `/Game/Blueprints/BP_BaseCharacter.Is_Boost` true _asbp_aiplayer))
    (:`NewEnumerator3`
      (set `/Game/Blueprints/BP_BaseCharacter.Is_Haste` true _asbp_aiplayer))))

(event `self.Shield.OnComponentEndOverlap`
  (params (OverlappedComponent :type "PrimitiveComponent Object Reference") (OtherActor :type "Actor Object Reference") (OtherComp :type "PrimitiveComponent Object Reference") (OtherBodyIndex :type Integer))
  ;[1 1 1] AOE Detection
  (bind _asbp_aiplayer (cast `/Game/Blueprints/AIPlayer/BP_AIPlayer` OtherActor))
  (set `/Game/Blueprints/BP_BaseCharacter.Is_Shield` false _asbp_aiplayer)
  (set `/Game/Blueprints/BP_BaseCharacter.Is_Boost` false _asbp_aiplayer)
  (set `/Game/Blueprints/BP_BaseCharacter.Is_Haste` false _asbp_aiplayer)
  (`BlueprintSetLibrary.Set_Remove` (`self.AllTargets`) _asbp_aiplayer))

(fn `UserConstructionScript`)