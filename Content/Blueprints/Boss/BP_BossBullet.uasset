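; BP_BossBullet is a boss projectile actor that damages characters it touches.
; Sphere1 overlaps ignore other boss bullets and act only on a BP_BaseCharacter that is not the bullet's Parent.
; A valid hit prints the character's name, applies fixed damage, spawns the P_BossExplosion effect slightly below the bullet and destroys it.
; Bullets that hit no valid character destroy themselves after a timed delay from BeginPlay.
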(event `self.ReceiveBeginPlay`
  (`KismetSystemLibrary.Delay` 20.0)
  (`self.K2_DestroyActor`))

(event `self.Sphere1.OnComponentBeginOverlap`
  (params (OverlappedComponent :type "PrimitiveComponent Object Reference") (OtherActor :type "Actor Object Reference") (OtherComp :type "PrimitiveComponent Object Reference") (OtherBodyIndex :type Integer) (bFromSweep :type Boolean) (SweepResult :type "HitResult Structure (by ref)"))
  (cast `/Game/Blueprints/Boss/BP_BossBullet` OtherActor
    (:`CastFailed`
      (bind _asbp_base_character (cast `/Game/Blueprints/BP_BaseCharacter` OtherActor))
      (if (!= _asbp_base_character (`self.Parent`))
        (`KismetSystemLibrary.PrintString` (`KismetSystemLibrary.GetDisplayName` _asbp_base_character))
        (`GameplayStatics.ApplyDamage` _asbp_base_character 20.0 (`AIBlueprintHelperLibrary.GetAIController` null) self "/Script/Engine.DamageType")
        (`NiagaraFunctionLibrary.SpawnSystemAtLocation` "/Game/RealtimePixelVFX/FX/P_BossExplosion.P_BossExplosion" (- (`self.K2_GetActorLocation`) (0.0 0.0 25.0)))
        (`self.K2_DestroyActor`)))))

(fn `UserConstructionScript`)