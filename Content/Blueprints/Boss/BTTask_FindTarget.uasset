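; Behavior Tree task for the boss that publishes its current target to the Blackboard.
; On execute, it casts the controlled pawn to BP_Boss and writes its Target into the TargetActor key, then finishes with success.
; A failed cast stops without finishing the task.
; Leftover unused nodes would randomly pick an AI player or the human player, but they are not wired in.
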(event `self.ReceiveExecuteAI`
  (params (OwnerController :type "AIController Object Reference") (ControlledPawn :type "Pawn Object Reference"))
  (bind _asbp_boss (cast `/Game/Blueprints/Boss/BP_Boss` ControlledPawn))
  (`BTFunctionLibrary.SetBlackboardValueAsObject` (make `BlackboardKeySelector` :`SelectedKeyName` "TargetActor") (`/Game/Blueprints/Boss/BP_Boss.Target` _asbp_boss))
  (`self.FinishExecute` true))