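; BP_MainPlayer is the player character, a flipbook sprite that moves along world X and Y from two input axes.
; Each tick it swaps between Walking and Idle flipbooks based on velocity.
; The MoveRight axis also triggers a flip that sets the tilted sprite's relative rotation by the sign of X velocity, mirroring it to face the travel direction.
; Controller-rotation flip nodes remain but never run.
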(event `InputAxis|MoveRight`
  (params (AxisValue :type "Float (single-precision)"))
  ;[1 1 1] Input
  (`self.AddMovementInput` (1.0 0.0 0.0) AxisValue)
  (`self.Flip_Animation`))

(event `self.ReceiveTick`
  (params (DeltaSeconds :type "Float (single-precision)"))
  (`self.Animation`))

(event `InputAxis|Move Forward / Backward`
  (params (AxisValue :type "Float (single-precision)"))
  ;[1 1 1] Input
  (`self.AddMovementInput` (0.0 1.0 0.0) (* AxisValue -1.0)))

(event `Animation`
  ;[1 1 1] Animations
  (`PaperFlipbookComponent.SetFlipbook` (`self.Sprite`) (select `bool` (> (`KismetMathLibrary.VSize` (`MovementComponent.Velocity` (`self.CharacterMovement`))) 0.0) :`false` "/Game/sprites(itch)/characters/Idle/Idle.Idle" :`true` "/Game/sprites(itch)/characters/Walking/Walking.Walking" :!type "PaperFlipbook Object Reference")))

(event `Flip_Animation`
  (bind _sprite (`self.Sprite`))
  ;[1 1 1] Animations
  (`/Engine/EditorBlueprintResources/StandardMacros.IsValid` (`self.GetController`)
    (:`Is Valid`
      (`/Engine/EditorBlueprintResources/StandardMacros.CompareFloat` (.x (`MovementComponent.Velocity` (`self.CharacterMovement`)))
        (:`>`
          (`SceneComponent.K2_SetRelativeRotation` _sprite (struct :`Roll` -30.0) false false))
        (:`<`
          (`SceneComponent.K2_SetRelativeRotation` _sprite (struct :`Yaw` 180.0 :`Roll` 30.0) false false))))))

(fn `UserConstructionScript`)